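; BP_Window is a window that spawns BP_Zombie at its spawn point at night unless it is boarded up.
; Tick shows the boards and refills their HP once when BoardedUp is set, and hides them when cleared.
; A delta-scaled random roll on Tick triggers SpawnZombie, which waits a random delay before checking ZombieMode's NightTime and spawning.
; Logic that wears boards down at night and breaks them with a sound is disconnected.
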(event Custom|SpawnZombie
  (bind _aszombie_mode (Utilities|Casting|CastToZombieMode (Game|GetGameMode)))
  (Utilities|FlowControl|Delay (Math|Random|RandomFloatinRange (Variables|Default|GetMinSpawnTime) (Variables|Default|GetMaxSpawnTime)))
  (if (and (not (Variables|Default|GetBoardedUp)) (Variables|/Game/Gameplay/ZombieMode.ZombieMode_C|GetNightTime _aszombie_mode))
    (Game|SpawnActorfromClass "/Game/Blueprints/Zombie/BP_Zombie.BP_Zombie_C" (Math|Transform|MakeTransform (.location (Transformation|GetWorldTransform (Variables|Default|GetSpawnPoint))) "0, 0, 0" "1,1,1") "AdjustIfPossibleButAlwaysSpawn" 0 0)))

(event EventBeginPlay)

(event Collision|EventActorBeginOverlap
  (params (OtherActor :type Actor%20Object%20Reference)))

(event EventTick
  (params (DeltaSeconds :type Float%20%28single-precision%29))
  (bind _boards (Variables|Default|GetBoards))
  (Utilities|FlowControl|Sequence
    (:then_0
      (if (Variables|Default|GetBoardedUp)
        (|DoOnceMultiInput :!label _label
          (:A%20Out
            (Rendering|SetVisibility _boards true true)
            (Variables|Default|SetBoardHP 1e+02))
          (:Reset%20Out
            (Rendering|SetVisibility _boards false true)))
        (else
          (goto _label Reset%20In))))
    (:then_1
      (if (< (Math|Random|RandomFloat) (* DeltaSeconds 0.05))
        (CallFunction|SpawnZombie)))))

(fn ConstructionScript)