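; BP_Grenade is a thrown grenade projectile with a short timed fuse that damages zombies within its blast radius.
; ExplosionRadius overlap events keep a list of the BP_Zombie actors currently in range.
; Tick counts the time alive and, once the fuse expires, a DoOnce plays the sound and effect, damages every listed zombie with the player character as damage causer, then destroys the grenade after a brief delay.
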(event OnComponentBeginOverlap(ExplosionRadius)
  (params (OverlappedComponent :type Primitive%20Component%20Object%20Reference) (OtherActor :type Actor%20Object%20Reference) (OtherComp :type Primitive%20Component%20Object%20Reference) (OtherBodyIndex :type Integer) (bFromSweep :type Boolean) (SweepResult :type Hit%20Result%20Structure%20%28by%20ref%29))
  (bind _asbp_zombie (Utilities|Casting|CastToBP_Zombie OtherActor))
  (Utilities|Array|AddUnique (Variables|Default|GetHurtList) _asbp_zombie))

(event OnComponentEndOverlap(ExplosionRadius)
  (params (OverlappedComponent :type Primitive%20Component%20Object%20Reference) (OtherActor :type Actor%20Object%20Reference) (OtherComp :type Primitive%20Component%20Object%20Reference) (OtherBodyIndex :type Integer))
  (bind _asbp_zombie (Utilities|Casting|CastToBP_Zombie OtherActor))
  (Utilities|Array|RemoveItem (Variables|Default|GetHurtList) _asbp_zombie))

(event EventBeginPlay
  (Components|Movement|SetUpdatedComponent (Variables|Default|GetProjectileMovement) (Variables|Default|GetSphere)))

(event EventTick
  (params (DeltaSeconds :type Float%20%28single-precision%29))
  (Variables|Default|SetTimeAlive (+ (Variables|Default|GetTimeAlive) DeltaSeconds))
  (if (> (Variables|Default|GetTimeAlive) 1.5)
    (Utilities|FlowControl|DoOnce false
      (:Completed
        (Audio|PlaySoundatLocation "/Game/Sounds/grenade_explosion.grenade_explosion" (Transformation|GetWorldLocation (Variables|Default|GetStaticMesh)) "0, 0, 0" 1.0 1.0 0.0 0 0 0)
        (Components|Activation|Activate (Variables|Default|GetExplosion) true)
        (for _array_element (Variables|Default|GetHurtList)
          (Game|Damage|ApplyDamage _array_element (Variables|Default|GetGrenadeDamage) 0 (Game|GetPlayerCharacter 0)))
        (Utilities|FlowControl|Delay 0.2)
        (Actor|DestroyActor)))))

(fn ConstructionScript)