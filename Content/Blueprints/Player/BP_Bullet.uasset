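; BP_Bullet is a projectile actor that damages zombies on contact.
; On spawn it sets its Box as the moving component, plays a gunshot sound and starts a limited lifespan.
; A Box overlap with BP_Zombie applies damage credited to the player character and destroys the bullet, if still enabled.
; A bounce disables damage, plays a ricochet sound and switches the Box to query-only collision.
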(event OnComponentBeginOverlap(Box)
  (params (OverlappedComponent :type Primitive%20Component%20Object%20Reference) (OtherActor :type Actor%20Object%20Reference) (OtherComp :type Primitive%20Component%20Object%20Reference) (OtherBodyIndex :type Integer) (bFromSweep :type Boolean) (SweepResult :type Hit%20Result%20Structure%20%28by%20ref%29))
  (bind _asbp_zombie (Utilities|Casting|CastToBP_Zombie OtherActor))
  (if (Variables|Default|GetEnabled)
    (Game|Damage|ApplyDamage _asbp_zombie (Variables|Default|GetDamage) 0 (Game|GetPlayerCharacter 0))
    (Actor|DestroyActor)))

(event OnProjectileBounce(ProjectileMovement)
  (params (ImpactResult :type Hit%20Result%20Structure%20%28by%20ref%29) (ImpactVelocity :type Vector%20%28by%20ref%29 :default "0, 0, 0"))
  (Variables|Default|SetEnabled false)
  (Audio|PlaySoundatLocation "/Game/Sounds/Bullet_Bounce_Cue.Bullet_Bounce_Cue" (Transformation|GetWorldLocation (Variables|Default|GetStaticMesh)) "0, 0, 0" 1.0 1.0 0.0 0 0 0)
  (Collision|SetCollisionEnabled (Variables|Default|GetBox) "QueryOnly"))

(event EventBeginPlay
  (Components|Movement|SetUpdatedComponent (Variables|Default|GetProjectileMovement) (Variables|Default|GetBox))
  (Audio|PlaySoundatLocation "/Game/Sounds/Gun/Gun_Shoot_Cue.Gun_Shoot_Cue" (Transformation|GetActorLocation) "0, 0, 0" 1.0 1.0 0.0 0 0 0)
  (Actor|SetLifeSpan 15.0))

(fn ConstructionScript)