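; BP_Friend is a friend actor with a health pool that gives audio feedback when hurt or killed.
; AnyDamage plays an impact cue at the actor's location, then subtracts the damage from CurrentHP, clamped between zero and MaxHP.
; At zero HP, a short delay precedes the death cue; the Blueprint neither destroys the actor nor guards against further hits retriggering that sound.
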(event EventBeginPlay)

(event Collision|EventActorBeginOverlap
  (params (OtherActor :type Actor%20Object%20Reference)))

(event EventTick
  (params (DeltaSeconds :type Float%20%28single-precision%29)))

(event Game|Damage|EventAnyDamage
  (params (Damage :type Float%20%28single-precision%29) (DamageType :type Damage%20Type%20Object%20Reference) (InstigatedBy :type Controller%20Object%20Reference) (DamageCauser :type Actor%20Object%20Reference))
  (Audio|PlaySoundatLocation "/Game/Sounds/Friend_Impact_Cue.Friend_Impact_Cue" (Transformation|GetActorLocation) "0, 0, 0" 1.0 1.0 0.0 0 0 0)
  (bind _output_get (Variables|Default|SetCurrentHP (Math|Float|Clamp(Float) (- (Variables|Default|GetCurrentHP) Damage) 0.0 (Variables|Default|GetMaxHP))))
  (if (not (> _output_get 0.0))
    (Utilities|FlowControl|Delay 0.2)
    (Audio|PlaySoundatLocation "/Game/Sounds/Friend_Death_Cue.Friend_Death_Cue" (Transformation|GetActorLocation) "0, 0, 0" 1.0 1.0 0.0 0 0 0)))

(fn ConstructionScript)