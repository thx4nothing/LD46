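; Zombie enemy that attacks the player and a friend character, with randomized starting health.
; AI perception and a per-tick range check write Targeted and InRange blackboard keys for its AI.
; Attack events apply damage within melee range, throttled by DoOnce and Delay cooldowns; idle sounds loop at random intervals.
; Damage triggers blood and sounds; death destroys it and credits a kill, but only when the player is the damage causer.
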(event OnTargetPerceptionUpdated(AIPerception)
  (params (Actor :type Actor%20Object%20Reference) (Stimulus :type AI%20Stimulus%20Structure))
  (AI|Components|Blackboard|SetValueasBool (AI|GetBlackboard 0) (Utilities|Name|MakeLiteralName "Targeted") (.bSuccessfullySensed (Utilities|Struct|BreakAIStimulus Stimulus))))

(event Custom|AttackPlayer
  (bind _asbp_player (Utilities|Casting|CastToBP_Player (Game|Player|GetPlayerPawn 0)))
  (if (< (Transformation|GetDistanceTo _asbp_player) (Variables|Default|GetMinAttackRange))
    (Utilities|FlowControl|DoOnce false :!label _label
      (:Completed
        (Game|Damage|ApplyDamage _asbp_player (Variables|Default|GetZombieDamage) 0 self)
        (Audio|PlaySoundatLocation "/Game/Sounds/Zombie/Zombie_Attack_Cue.Zombie_Attack_Cue" (Transformation|GetActorLocation) "0, 0, 0" 1.0 1.0 0.0 0 0 0)
        (Utilities|FlowControl|Delay 0.75)
        (goto _label Reset)))))

(event Custom|AttackFriend
  (bind _friend (Variables|Default|GetFriend))
  (if (< (Transformation|GetDistanceTo _friend) (Variables|Default|GetMinAttackRange))
    (Utilities|FlowControl|DoOnce false :!label _label
      (:Completed
        (Game|Damage|ApplyDamage _friend (Variables|Default|GetZombieDamage) 0 self)
        (Audio|PlaySoundatLocation "/Game/Sounds/Zombie/Zombie_Attack_Cue.Zombie_Attack_Cue" (Transformation|GetActorLocation) "0, 0, 0" 1.0 1.0 0.0 0 0 0)
        (Utilities|FlowControl|Delay 0.75)
        (goto _label Reset)))))

(event EventBeginPlay
  (bind _output_get (Variables|Default|SetCurrentHP (Math|Random|RandomFloatinRange 4.0 9.0)))
  (Variables|Default|SetMaxHP _output_get)
  (bind _outactors (Actor|GetAllActorsOfClass "/Game/Blueprints/Friend/BP_Friend.BP_Friend_C"))
  (Variables|Default|SetFriend (Utilities|Array|Get(acopy) _outactors)))

(event Game|Damage|EventAnyDamage
  (params (Damage :type Float%20%28single-precision%29) (DamageType :type Damage%20Type%20Object%20Reference) (InstigatedBy :type Controller%20Object%20Reference) (DamageCauser :type Actor%20Object%20Reference))
  (bind _returnvalue (Transformation|GetActorLocation))
  (Components|Activation|Activate (Variables|Default|GetP_Blood) true)
  (bind _output_get (Variables|Default|SetCurrentHP (Math|Float|Clamp(Float) (- (Variables|Default|GetCurrentHP) Damage) 0.0 (Variables|Default|GetMaxHP))))
  (if (> _output_get 0.0)
    (Audio|PlaySoundatLocation "/Game/Sounds/Zombie/Zombie_Impact_Cue.Zombie_Impact_Cue" _returnvalue "0, 0, 0" 1.0 1.0 0.0 0 0 0)
    (else
      (Audio|PlaySoundatLocation "/Game/Sounds/Zombie/Zombie_Death_Cue.Zombie_Death_Cue" _returnvalue "0, 0, 0" 1.0 1.0 0.0 0 0 0)
      (bind _asbp_player (Utilities|Casting|CastToBP_Player DamageCauser))
      (Math|Integer|IncrementInt (Variables|/Game/Blueprints/Player/BP_Player.BP_Player_C|GetKills _asbp_player)
        (:%20%20
          (Actor|DestroyActor))))))

(event EventTick
  (params (DeltaSeconds :type Float%20%28single-precision%29))
  (Utilities|FlowControl|Sequence
    (:then_0
      (AI|Components|Blackboard|SetValueasBool (AI|GetBlackboard 0) (Utilities|Name|MakeLiteralName "InRange") (CallFunction|InAttackRange)))
    (:then_1
      (Utilities|FlowControl|DoOnce false :!label _label
        (:Completed
          (Audio|PlaySoundatLocation "/Game/Sounds/Zombie/Zombie_Idle_Cue.Zombie_Idle_Cue" (Transformation|GetActorLocation) "0, 0, 0" 1.0 1.0 0.0 0 0 0)
          (Utilities|FlowControl|Delay (Math|Random|RandomFloatinRange 2.0 8.0))
          (goto _label Reset))))))

(fn ConstructionScript)

(fn InAttackRange
  (bind _outactors (Actor|GetAllActorsOfClass "/Game/Blueprints/Friend/BP_Friend.BP_Friend_C"))
  (return (or (< (Transformation|GetDistanceTo (Game|Player|GetPlayerPawn 0)) (Variables|Default|GetMinAttackRange)) (< (Transformation|GetDistanceTo (Utilities|Array|Get(acopy) _outactors)) (Variables|Default|GetMinAttackRange)))))