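; Door actor that swings 90 degrees based on trigger occupancy and the night-time flag in ZombieMode.
; Box overlap events set PlayerInside for any actor, without filtering for the player.
; Tick rotates Scene +90 yaw when occupied at night and -90 otherwise.
; Two cross-resetting DoOnce gates limit rotation to one instant step per state change.
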(event OnComponentBeginOverlap(Box)
  (params (OverlappedComponent :type Primitive%20Component%20Object%20Reference) (OtherActor :type Actor%20Object%20Reference) (OtherComp :type Primitive%20Component%20Object%20Reference) (OtherBodyIndex :type Integer) (bFromSweep :type Boolean) (SweepResult :type Hit%20Result%20Structure%20%28by%20ref%29))
  (Variables|Default|SetPlayerInside true))

(event OnComponentEndOverlap(Box)
  (params (OverlappedComponent :type Primitive%20Component%20Object%20Reference) (OtherActor :type Actor%20Object%20Reference) (OtherComp :type Primitive%20Component%20Object%20Reference) (OtherBodyIndex :type Integer))
  (Variables|Default|SetPlayerInside false))

(event EventTick
  (params (DeltaSeconds :type Float%20%28single-precision%29))
  (bind _aszombie_mode (Utilities|Casting|CastToZombieMode (Game|GetGameMode)))
  (if (and (Variables|Default|GetPlayerInside) (Variables|/Game/Gameplay/ZombieMode.ZombieMode_C|GetNightTime _aszombie_mode))
    (Utilities|FlowControl|DoOnce true :!label _label
      (:Completed
        (Transformation|AddLocalRotation (Variables|Default|GetScene) "0,90.000000, 0" false false)
        (goto _label_2 Reset)))
    (else
      (Utilities|FlowControl|DoOnce false :!label _label_2
        (:Completed
          (Transformation|AddLocalRotation (Variables|Default|GetScene) "0,-90.000000, 0" false false)
          (goto _label Reset))))))

(fn ConstructionScript)